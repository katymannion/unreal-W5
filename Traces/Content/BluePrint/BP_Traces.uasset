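; BP_Traces is an actor that appears to be a test of box tracing.
; Each Tick it runs a Visibility box trace from its Arrow component's location with timed debug drawing, leaving the end point at its default.
; A forward-offset end point is computed but unused, and a hit-actor comparison that prints "Hello" is disconnected, so the trace result has no effect.
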(event `self.ReceiveTick`
  (params (DeltaSeconds :type "Float (single-precision)"))
  (bind _outhit (`KismetSystemLibrary.BoxTraceSingle` :`Start` (`SceneComponent.K2_GetComponentLocation` (`self.Arrow`)) :`TraceChannel` "TraceTypeQuery1" :`DrawDebugType` "ForDuration")))

(fn `UserConstructionScript`)